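; HiddenAreas is a Blueprint that hides and reveals a Paper2D tile map through two overlap triggers, Visible and Invisible.
; Overlapping Visible hides the tile map and the trigger, disables the tile map's collision and enables query-and-physics collision on Invisible.
; Overlapping Invisible makes the tile map visible again but leaves its collision disabled.
; Neither handler filters the overlapping actor.
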(event `self.Visible.OnComponentBeginOverlap`
  (params (OverlappedComponent :type "PrimitiveComponent Object Reference") (OtherActor :type "Actor Object Reference") (OtherComp :type "PrimitiveComponent Object Reference") (OtherBodyIndex :type Integer) (bFromSweep :type Boolean) (SweepResult :type "HitResult Structure (by ref)"))
  (bind _output_get (set `self.IsVisible` false))
  (`SceneComponent.SetVisibility` OverlappedComponent _output_get false)
  (`SceneComponent.SetVisibility` (`self.PaperTileMap`) _output_get false)
  (`PrimitiveComponent.SetCollisionEnabled` (`self.PaperTileMap`) "NoCollision")
  (`PrimitiveComponent.SetCollisionEnabled` (`self.Invisible`) "QueryAndPhysics"))

(event `self.Invisible.OnComponentBeginOverlap`
  (params (OverlappedComponent :type "PrimitiveComponent Object Reference") (OtherActor :type "Actor Object Reference") (OtherComp :type "PrimitiveComponent Object Reference") (OtherBodyIndex :type Integer) (bFromSweep :type Boolean) (SweepResult :type "HitResult Structure (by ref)"))
  (bind _output_get (set `self.IsVisible` true))
  (`SceneComponent.SetVisibility` (`self.PaperTileMap`) _output_get false))

(fn `UserConstructionScript`
  (`parent.UserConstructionScript`))