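; Ladder actor that switches the player character into a climbing state through overlap events.
; On overlap begin it flags the player as on the ladder and, only if W is held at that moment, sets Flying movement and applies one upward input.
; On overlap end it clears the flag and sets Falling.
; There is no per-frame climb logic here, and the flag is never read in this graph.
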(event `self.ReceiveActorBeginOverlap`
  (params (OtherActor :type "Actor Object Reference"))
  (bind _returnvalue (`GameplayStatics.GetPlayerPawn` 0))
  (bind _asplayer_character_blueprint (cast `/Game/Assets/Blueprints/PlayerCharacterBlueprint` OtherActor))
  (set `self.IsPlayerOnLadder` true)
  (if (`PlayerController.IsInputKeyDown` (`GameplayStatics.GetPlayerController` 0) "W")
    (`CharacterMovementComponent.SetMovementMode` (`Character.CharacterMovement` _asplayer_character_blueprint) "MOVE_Flying" 0)
    (`Pawn.AddMovementInput` _returnvalue (`self.GetActorUpVector` _returnvalue) 1.0 false)))

(event `self.ReceiveActorEndOverlap`
  (params (OtherActor :type "Actor Object Reference"))
  (bind _asplayer_character_blueprint (cast `/Game/Assets/Blueprints/PlayerCharacterBlueprint` OtherActor))
  (set `self.IsPlayerOnLadder` false)
  (`CharacterMovementComponent.SetMovementMode` (`Character.CharacterMovement` _asplayer_character_blueprint) "MOVE_Falling" 0))

(fn `UserConstructionScript`
  (`parent.UserConstructionScript`))