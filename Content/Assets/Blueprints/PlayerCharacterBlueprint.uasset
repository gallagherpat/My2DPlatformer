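; Player character for a 2D flipbook side-scroller, handling movement, jumping, death and respawn.
; Tick picks the death, jump, move or idle flipbook and flips controller yaw from X velocity, using the last input direction when stopped.
; Axis inputs add horizontal and vertical movement, with vertical input also referencing a ladder flag.
; Any damage disables movement, waits out the death animation, then returns the player to the BeginPlay location.
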(event `self.ReceiveTick`
  (params (DeltaSeconds :type "Float (single-precision)"))
  ;[1 1 1] Event Tick
  (`self.HandleAnim`)
  (`self.HandleRotation`))

(event `InputAction|Jump`
  (params (Key :type "Key Structure"))
  ;[1 1 1] Jumping Handle
  (:`Pressed`
    (`self.Jump`))
  (:`Released`
    (`self.StopJumping`)))

(event `HandleAnim`
  (bind _sprite (`self.Sprite`))
  ;[1 1 1] Animation Controller
  (if (`self.isDead`)
    (`PaperFlipbookComponent.SetFlipbook` (`self.Sprite`) (`self.playerDeathAnim`))
    (elif (`NavMovementComponent.IsFalling` (`self.CharacterMovement`))
      (`PaperFlipbookComponent.SetFlipbook` _sprite "/Game/Assets/Characters/Jumping_Anim.Jumping_Anim")
      (else
        (`PaperFlipbookComponent.SetFlipbook` _sprite (select `bool` (> (`KismetMathLibrary.VSize` (`MovementComponent.Velocity` (`self.CharacterMovement`))) 0.0) :`false` "/Game/Assets/Characters/Idle_Anim.Idle_Anim" :`true` "/Game/Assets/Characters/Moving_Anim.Moving_Anim" :!type "PaperFlipbook Object Reference"))))))

(event `InputAxis|MoveRight`
  (params (AxisValue :type "Float (single-precision)"))
  ;[1 1 1] Movement Controller
  (if (> AxisValue 0.0)
    (set `self.isMovingRight` true)
    (elif (< AxisValue 0.0)
      (set `self.isMovingRight` false)))
  (`self.AddMovementInput` (0.6 0.0 0.0) AxisValue))

(event `InputAxis|MoveUp`
  (params (AxisValue :type "Float (single-precision)"))
  ;[1 1 1] Movement Controller
  (if (> AxisValue 0.0)
    (set `self.isMovingUp` true)
    (if (`/Game/Assets/Blueprints/Ladder.IsPlayerOnLadder` (`self.Target`)) :!label _label
      _
      (else
        _))
    (`self.Jump`)
    (elif (< AxisValue 0.0)
      (set `self.isMovingUp` false)
      (goto _label)
      (else
        _)))
  (`self.AddMovementInput` (0.0 0.0 0.5) AxisValue))

(event `HandleRotation`
  (bind _velocity_x (`KismetMathLibrary.BreakVector` (`MovementComponent.Velocity` (`self.CharacterMovement`))))
  ;[1 1 1] Handle Camera/player rotation
  (`/Engine/EditorBlueprintResources/StandardMacros.CompareFloat` _velocity_x
    (:`>`
      (`Controller.SetControlRotation` (`self.GetController`) (`KismetMathLibrary.MakeRotator` 0.0 0.0 180.0) :!label _label_2))
    (:`==`
      (if (`self.isMovingRight`)
        (goto _label_2)
        (else
          (`Controller.SetControlRotation` (`self.GetController`) (`KismetMathLibrary.MakeRotator` 0.0) :!label _label_3))))
    (:`<`
      (goto _label_3))))

(event `self.ReceiveAnyDamage`
  (params (Damage :type "Float (single-precision)") (DamageType :type "DamageType Object Reference") (InstigatedBy :type "Controller Object Reference") (DamageCauser :type "Actor Object Reference"))
  ;[1 1 1] Damage Handler
  (set `self.isDead` true)
  (`ActorComponent.SetActive` (`self.CharacterMovement`) false false)
  (`KismetSystemLibrary.Delay` (- (`PaperFlipbook.GetTotalDuration` (`self.playerDeathAnim`)) 0.1))
  (`self.RespawnPlayerCharacter`))

(event `self.ReceiveBeginPlay`
  ;[1 1 1] Get Player starting location
  (set `self.respawnLocation` (`self.K2_GetActorLocation`)))

(event `RespawnPlayerCharacter`
  ;[1 1 1] Respawn player
  (`self.K2_SetActorLocation` (`self.respawnLocation`))
  (set `self.isDead` false)
  (`ActorComponent.SetActive` (`self.CharacterMovement`) true false))

(fn `UserConstructionScript`)