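; Teleport trigger actor that moves the player to a fixed height when they enter its box.
; On overlap with the referenced player character, it shows a smoke flipbook and waits briefly.
; It then teleports the player to that height, keeping their current X, Y and rotation, and clears the flipbook.
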(event `self.Box.OnComponentBeginOverlap`
  (params (OverlappedComponent :type "PrimitiveComponent Object Reference") (OtherActor :type "Actor Object Reference") (OtherComp :type "PrimitiveComponent Object Reference") (OtherBodyIndex :type Integer) (bFromSweep :type Boolean) (SweepResult :type "HitResult Structure (by ref)"))
  (bind _playercharacterref (`self.PlayerCharacterRef`))
  (bind (_returnvalue_x _returnvalue_y) (`KismetMathLibrary.BreakVector` (`self.K2_GetActorLocation` _playercharacterref)))
  (if (== OtherActor _playercharacterref)
    (`PaperFlipbookComponent.SetFlipbook` (`self.PaperFlipbook`) "/Game/Assets/Smoke/Smoke_Flipbook.Smoke_Flipbook")
    (`KismetSystemLibrary.Delay` 0.2)
    (`self.K2_TeleportTo` _playercharacterref (`KismetMathLibrary.MakeVector` _returnvalue_x _returnvalue_y 200.0) (`self.K2_GetActorRotation` _playercharacterref))
    (`PaperFlipbookComponent.SetFlipbook` (`self.PaperFlipbook`) null)))

(fn `UserConstructionScript`
  (`parent.UserConstructionScript`))