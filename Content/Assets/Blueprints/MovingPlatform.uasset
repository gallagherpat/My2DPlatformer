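; A moving platform actor that shuttles its Paper2D sprite back and forth between End and Start points.
; BeginPlay waits briefly, then runs an endless latent loop of MoveComponentTo calls with pauses at each end, using each marker component's relative location as the target.
; The initial SetWorldLocation reassigns the sprite's current position; Tick and the construction script only call their parents.
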(event `self.ReceiveBeginPlay`
  (bind _returnvalue_location (`KismetMathLibrary.BreakTransform` (`SceneComponent.GetRelativeTransform` (`self.Start`))))
  (bind _returnvalue_location_2 (`KismetMathLibrary.BreakTransform` (`SceneComponent.GetRelativeTransform` (`self.End`))))
  (`parent.ReceiveBeginPlay`)
  (`SceneComponent.K2_SetWorldLocation` (`self.PaperSprite`) (`SceneComponent.K2_GetComponentLocation` (`self.PaperSprite`)) false false)
  (`KismetSystemLibrary.Delay` 0.75)
  (`KismetSystemLibrary.MoveComponentTo` (`self.PaperSprite`) _returnvalue_location_2 (struct) false false 2.0 :!label _label)
  (`KismetSystemLibrary.Delay` 1.5)
  (`KismetSystemLibrary.MoveComponentTo` (`self.PaperSprite`) _returnvalue_location (struct) false false 2.0)
  (`KismetSystemLibrary.Delay` 1.5)
  (goto _label))

(event `self.ReceiveTick`
  (params (DeltaSeconds :type "Float (single-precision)"))
  (`parent.ReceiveTick` DeltaSeconds))

(fn `UserConstructionScript`
  (`parent.UserConstructionScript`))